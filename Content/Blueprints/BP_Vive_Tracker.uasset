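; Vive Tracker actor that drives a camera from SteamVR tracking data so virtual movement matches real space.
; BeginPlay enables player input on the Camera and makes it the view target.
; Each Tick it applies the pose of every "Other" tracked device to the Camera root's relative transform, so the last one wins.
; Position and rotation axes are swapped and partly negated, after adding XRotComp and YRotComp rotation offsets.
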(event EventBeginPlay
  (bind _returnvalue (Game|GetPlayerController 0))
  (bind _camera (Variables|Default|GetCamera))
  ;[0.2898 0.9502 1] Setter camera til å få Player Input
  (Input|EnableInput _camera _returnvalue)
  (Game|Player|SetViewTargetwithBlend _returnvalue _camera 0.0 "VTBlend_Linear" 0.0 false))

(event EventTick
  (params (DeltaSeconds :type Float%20%28single-precision%29))
  ;[1 1 1] Henter ID til Vive Controller
  (for _array_element (Class|SteamVRFunctionLibrary|GetValidTrackedDeviceIds "Other")
    ;[1 1 1] Setter ny posisjon og rotasjon på Actor
    (Transformation|SetRelativeLocationAndRotation (Variables|/Script/Engine.Actor|GetRootComponent (Variables|Default|GetCamera)) (Math|Vector|MakeVector (.y (.location (Math|Transform|MakeTransform (.OutPosition (Class|SteamVRFunctionLibrary|GetTrackedDevicePositionandOrientation _array_element)) (.OutOrientation (Class|SteamVRFunctionLibrary|GetTrackedDevicePositionandOrientation _array_element))))) (* (.x (.location (Math|Transform|MakeTransform (.OutPosition (Class|SteamVRFunctionLibrary|GetTrackedDevicePositionandOrientation _array_element)) (.OutOrientation (Class|SteamVRFunctionLibrary|GetTrackedDevicePositionandOrientation _array_element))))) -1.0) (.z (.location (Math|Transform|MakeTransform (.OutPosition (Class|SteamVRFunctionLibrary|GetTrackedDevicePositionandOrientation _array_element)) (.OutOrientation (Class|SteamVRFunctionLibrary|GetTrackedDevicePositionandOrientation _array_element)))))) (Math|Rotator|MakeRotator (.pitch (Math|Rotator|CombineRotators (Math|Rotator|MakeRotator (.roll (.rotation (Math|Transform|MakeTransform (.OutPosition (Class|SteamVRFunctionLibrary|GetTrackedDevicePositionandOrientation _array_element)) (.OutOrientation (Class|SteamVRFunctionLibrary|GetTrackedDevicePositionandOrientation _array_element))))) (.pitch (.rotation (Math|Transform|MakeTransform (.OutPosition (Class|SteamVRFunctionLibrary|GetTrackedDevicePositionandOrientation _array_element)) (.OutOrientation (Class|SteamVRFunctionLibrary|GetTrackedDevicePositionandOrientation _array_element))))) (.yaw (.rotation (Math|Transform|MakeTransform (.OutPosition (Class|SteamVRFunctionLibrary|GetTrackedDevicePositionandOrientation _array_element)) (.OutOrientation (Class|SteamVRFunctionLibrary|GetTrackedDevicePositionandOrientation _array_element)))))) (Math|Rotator|MakeRotator (Variables|Default|GetXRotComp) (Variables|Default|GetYRotComp) 0.0))) (.yaw (Math|Rotator|CombineRotators (Math|Rotator|MakeRotator (.roll (.rotation (Math|Transform|MakeTransform (.OutPosition (Class|SteamVRFunctionLibrary|GetTrackedDevicePositionandOrientation _array_element)) (.OutOrientation (Class|SteamVRFunctionLibrary|GetTrackedDevicePositionandOrientation _array_element))))) (.pitch (.rotation (Math|Transform|MakeTransform (.OutPosition (Class|SteamVRFunctionLibrary|GetTrackedDevicePositionandOrientation _array_element)) (.OutOrientation (Class|SteamVRFunctionLibrary|GetTrackedDevicePositionandOrientation _array_element))))) (.yaw (.rotation (Math|Transform|MakeTransform (.OutPosition (Class|SteamVRFunctionLibrary|GetTrackedDevicePositionandOrientation _array_element)) (.OutOrientation (Class|SteamVRFunctionLibrary|GetTrackedDevicePositionandOrientation _array_element)))))) (Math|Rotator|MakeRotator (Variables|Default|GetXRotComp) (Variables|Default|GetYRotComp) 0.0))) (* (.roll (Math|Rotator|CombineRotators (Math|Rotator|MakeRotator (.roll (.rotation (Math|Transform|MakeTransform (.OutPosition (Class|SteamVRFunctionLibrary|GetTrackedDevicePositionandOrientation _array_element)) (.OutOrientation (Class|SteamVRFunctionLibrary|GetTrackedDevicePositionandOrientation _array_element))))) (.pitch (.rotation (Math|Transform|MakeTransform (.OutPosition (Class|SteamVRFunctionLibrary|GetTrackedDevicePositionandOrientation _array_element)) (.OutOrientation (Class|SteamVRFunctionLibrary|GetTrackedDevicePositionandOrientation _array_element))))) (.yaw (.rotation (Math|Transform|MakeTransform (.OutPosition (Class|SteamVRFunctionLibrary|GetTrackedDevicePositionandOrientation _array_element)) (.OutOrientation (Class|SteamVRFunctionLibrary|GetTrackedDevicePositionandOrientation _array_element)))))) (Math|Rotator|MakeRotator (Variables|Default|GetXRotComp) (Variables|Default|GetYRotComp) 0.0))) -1.0)) false false)))