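; Stage controller Blueprint that drives a TrackerCamera component from VR tracked devices, likely for a virtual camera on a stage.
; One custom event enables player 0's input and sets that player's view target.
; Another applies each "Other"-type device's pose to the camera's relative transform, so the last one wins.
; It swaps and negates axes to remap the pose, adding XRotComp and YRotComp as rotation offsets.
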(event Custom|CustomEvent
  (bind _returnvalue (Game|GetPlayerController 0))
  (Input|EnableInput _returnvalue)
  (Game|Player|SetViewTargetwithBlend _returnvalue 0 0.0 "VTBlend_Linear" 0.0 false))

(event Custom|CustomEvent_1
  (params (DeltaSeconds :type Float%20%28single-precision%29))
  (for _array_element (Class|SteamVRFunctionLibrary|GetValidTrackedDeviceIds "Other")
    (Transformation|SetRelativeLocationAndRotation (Variables|Default|GetTrackerCamera) (Math|Vector|MakeVector (.y (.location (Math|Transform|MakeTransform (.OutPosition (Class|SteamVRFunctionLibrary|GetTrackedDevicePositionandOrientation _array_element)) (.OutOrientation (Class|SteamVRFunctionLibrary|GetTrackedDevicePositionandOrientation _array_element))))) (* (.x (.location (Math|Transform|MakeTransform (.OutPosition (Class|SteamVRFunctionLibrary|GetTrackedDevicePositionandOrientation _array_element)) (.OutOrientation (Class|SteamVRFunctionLibrary|GetTrackedDevicePositionandOrientation _array_element))))) -1.0) (.z (.location (Math|Transform|MakeTransform (.OutPosition (Class|SteamVRFunctionLibrary|GetTrackedDevicePositionandOrientation _array_element)) (.OutOrientation (Class|SteamVRFunctionLibrary|GetTrackedDevicePositionandOrientation _array_element)))))) (Math|Rotator|MakeRotator (.pitch (Math|Rotator|CombineRotators (Math|Rotator|MakeRotator (.roll (.rotation (Math|Transform|MakeTransform (.OutPosition (Class|SteamVRFunctionLibrary|GetTrackedDevicePositionandOrientation _array_element)) (.OutOrientation (Class|SteamVRFunctionLibrary|GetTrackedDevicePositionandOrientation _array_element))))) (.pitch (.rotation (Math|Transform|MakeTransform (.OutPosition (Class|SteamVRFunctionLibrary|GetTrackedDevicePositionandOrientation _array_element)) (.OutOrientation (Class|SteamVRFunctionLibrary|GetTrackedDevicePositionandOrientation _array_element))))) (.yaw (.rotation (Math|Transform|MakeTransform (.OutPosition (Class|SteamVRFunctionLibrary|GetTrackedDevicePositionandOrientation _array_element)) (.OutOrientation (Class|SteamVRFunctionLibrary|GetTrackedDevicePositionandOrientation _array_element)))))) (Math|Rotator|MakeRotator (Variables|Default|GetXRotComp) (Variables|Default|GetYRotComp) 0.0))) (.yaw (Math|Rotator|CombineRotators (Math|Rotator|MakeRotator (.roll (.rotation (Math|Transform|MakeTransform (.OutPosition (Class|SteamVRFunctionLibrary|GetTrackedDevicePositionandOrientation _array_element)) (.OutOrientation (Class|SteamVRFunctionLibrary|GetTrackedDevicePositionandOrientation _array_element))))) (.pitch (.rotation (Math|Transform|MakeTransform (.OutPosition (Class|SteamVRFunctionLibrary|GetTrackedDevicePositionandOrientation _array_element)) (.OutOrientation (Class|SteamVRFunctionLibrary|GetTrackedDevicePositionandOrientation _array_element))))) (.yaw (.rotation (Math|Transform|MakeTransform (.OutPosition (Class|SteamVRFunctionLibrary|GetTrackedDevicePositionandOrientation _array_element)) (.OutOrientation (Class|SteamVRFunctionLibrary|GetTrackedDevicePositionandOrientation _array_element)))))) (Math|Rotator|MakeRotator (Variables|Default|GetXRotComp) (Variables|Default|GetYRotComp) 0.0))) (* (.roll (Math|Rotator|CombineRotators (Math|Rotator|MakeRotator (.roll (.rotation (Math|Transform|MakeTransform (.OutPosition (Class|SteamVRFunctionLibrary|GetTrackedDevicePositionandOrientation _array_element)) (.OutOrientation (Class|SteamVRFunctionLibrary|GetTrackedDevicePositionandOrientation _array_element))))) (.pitch (.rotation (Math|Transform|MakeTransform (.OutPosition (Class|SteamVRFunctionLibrary|GetTrackedDevicePositionandOrientation _array_element)) (.OutOrientation (Class|SteamVRFunctionLibrary|GetTrackedDevicePositionandOrientation _array_element))))) (.yaw (.rotation (Math|Transform|MakeTransform (.OutPosition (Class|SteamVRFunctionLibrary|GetTrackedDevicePositionandOrientation _array_element)) (.OutOrientation (Class|SteamVRFunctionLibrary|GetTrackedDevicePositionandOrientation _array_element)))))) (Math|Rotator|MakeRotator (Variables|Default|GetXRotComp) (Variables|Default|GetYRotComp) 0.0))) -1.0)) false false)))

(fn ConstructionScript)